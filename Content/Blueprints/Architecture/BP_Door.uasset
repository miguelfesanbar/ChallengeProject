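; Door actor that swings open and closed when its DoorOpen event fires while the player is nearby.
; RoomCollision1 overlaps set a NextToTheDoor flag on the ThirdPersonCharacter, which DoorOpen checks on player 0.
; A FlipFlop alternately plays and reverses a timeline that drives the yaw of the Scene component.
; The proximity flag lives on the character, so the check does not identify which door is near.
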(event `self.RoomCollision1.OnComponentBeginOverlap`
  (params (OverlappedComponent :type "PrimitiveComponent Object Reference") (OtherActor :type "Actor Object Reference") (OtherComp :type "PrimitiveComponent Object Reference") (OtherBodyIndex :type Integer) (bFromSweep :type Boolean) (SweepResult :type "HitResult Structure (by ref)"))
  ;[0.1662 1 0.1656] Get closer to the door
  (bind _asthird_person_character (cast `/Game/Blueprints/Spawn/ThirdPersonCharacter` OtherActor))
  (set `/Game/Blueprints/Spawn/ThirdPersonCharacter.NextToTheDoor` true _asthird_person_character))

(event `self.RoomCollision1.OnComponentEndOverlap`
  (params (OverlappedComponent :type "PrimitiveComponent Object Reference") (OtherActor :type "Actor Object Reference") (OtherComp :type "PrimitiveComponent Object Reference") (OtherBodyIndex :type Integer))
  ;[1 0.1888 0.1749] Get away from the door
  (bind _asthird_person_character (cast `/Game/Blueprints/Spawn/ThirdPersonCharacter` OtherActor))
  (set `/Game/Blueprints/Spawn/ThirdPersonCharacter.NextToTheDoor` false _asthird_person_character))

(event `DoorOpen`
  ;[0.9674 1 0.29] Check and Open/Close the Door
  (if (`self.IsNextToTheDoor`)
    (`/Engine/EditorBlueprintResources/StandardMacros.FlipFlop`
      (:`A`
        (bind (_direction _dooropening) (`Timeline|DoorAnimationTimeline` :!label _label)
          (:`Update`
            (`self.MoveDoor` _dooropening))))
      (:`B`
        (goto _label :!via `Reverse`)))))

(fn `IsNextToTheDoor`
  (returns (IsNextToTheDoor :type Boolean))
  (bind _asthird_person_character (cast `/Game/Blueprints/Spawn/ThirdPersonCharacter` (`GameplayStatics.GetPlayerCharacter` 0)))
  (return (`/Game/Blueprints/Spawn/ThirdPersonCharacter.NextToTheDoor` _asthird_person_character)))

(fn `MoveDoor`
  (params (Yaw :type "Float (double-precision)"))
  (`SceneComponent.K2_SetRelativeRotation` (`self.Scene`) (`KismetMathLibrary.MakeRotator` 0.0 0.0 Yaw) false false))

(fn `UserConstructionScript`)